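; Main game mode for an Octo-versus-Hunters match, with the Octo spawned as a VR pawn.
; Login spawns and possesses pawns by role, and mid-game joiners get a free UID and skin from the GameInstance.
; Hunters use shuffled available respawn areas with a tagged fallback, and bullet damage is divided by the tracked player count.
; It also cleans up on logout and switches game state to GameOver, showing the result through the first player controller.
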(event Custom|SetNewClientUserInfo
  (params (PlayerState :type BP%20Main%20PS%20Object%20Reference))
  ;[1 1 1] 중간 난입한 플레이어 정보 세팅 (비어있는 UID와 skin을 지정해주고 그걸 다시 클라이언트한테 보내줌)
  (bind _asbp_gi (Utilities|Casting|CastToBP_GI (Game|GetGameInstance)))
  (Utilities|IsValid _asbp_gi
    (:Is%20Valid
      (bind _uid (Default|GetUIDMain _asbp_gi))
      (bind _skinstate (Default|GetSkin _asbp_gi _uid))
      (Default|SetLocalInfotoClientGI PlayerState _uid _skinstate)
      (Default|SetLocalInfoServer PlayerState))))

(event Custom|RespawnPawn
  (params (Hunter :type Pawn%20Object%20Reference))
  ;[1 1 1] 초기 폰 배치
  (Utilities|IsValid Hunter
    (:Is%20Valid
      (bind _respawntransform (CallFunction|GetHunterSpawnPoints))
      (Transformation|SetActorTransform Hunter _respawntransform))))

(event Custom|GameOver
  (params (IsHunterVictory :type Boolean))
  ;[1 1 1] 게임오버 처리
  (bind _asbp_main_gs (Utilities|Casting|CastToBP_MainGS (Game|GetGameState)))
  (if (Utilities|Enum|Equal(Enum) (Variables|/Script/OctoPrototype.MainGS|GetCurrentGameState _asbp_main_gs) "Playing")
    (Variables|/Script/OctoPrototype.MainGS|SetCurrentGameState _asbp_main_gs "GameOver")
    (Class|MainGS|DowhenCurrentGameStateChanged _asbp_main_gs)
    (if IsHunterVictory
      (CallFunction|HunterWin)
      (else
        (CallFunction|OctoWin)))))

(event Custom|OctoWin
  ;[1 1 1] 게임오버 처리
  ;;[1 1 1] 게임오버시 결과 화면 처리
  (bind _asbp_main_pc (Utilities|Casting|CastToBP_MainPC (Game|GetPlayerController 0)))
  (Default|ShowResult _asbp_main_pc false))

(event Custom|HunterWin
  ;[1 1 1] 게임오버 처리
  ;;[1 1 1] 게임오버시 결과 화면 처리
  (bind _asbp_main_pc (Utilities|Casting|CastToBP_MainPC (Game|GetPlayerController 0)))
  (Default|ShowResult _asbp_main_pc true))

(event Custom|SpawnHunter
  (params (PlayerController :type Player%20Controller%20Object%20Reference))
  (bind _playercount (Variables|Default|GetPlayerCount))
  ;[1 1 1] 헌터스폰
  (bind _asbp_main_pc (Utilities|Casting|CastToBP_MainPC PlayerController))
  (Utilities|IsValid _asbp_main_pc
    (:Is%20Valid
      (bind _asbp_gi (Utilities|Casting|CastToBP_GI (Game|GetGameInstance)))
      (bind _respawntransform (CallFunction|GetHunterSpawnPoints))
      (bind _returnvalue (Game|SpawnActorfromClass (Variables|/Game/Blueprints/Public/BP_GI.BP_GI_C|GetDefaultHunterClass _asbp_gi) _respawntransform "AlwaysSpawn" 0 0))
      (Pawn|Possess _asbp_main_pc _returnvalue)
      (Default|SetMeshandMaterialAllPlayersServer _asbp_main_pc)
      (Math|Integer|IncrementInt _playercount
        (:%20%20
          (if (!= _playercount 0)
            (Variables|Default|SetBulletDamage (/ (Variables|Default|GetBaseBulletDamage) (Math|Conversions|ToFloat(Integer) _playercount)))))))))

(event EventOnLogout
  (params (ExitingController :type Controller%20Object%20Reference))
  (bind _playercount (Variables|Default|GetPlayerCount))
  ;[1 1 1] 로그아웃 처리
  (bind _asbp_main_ps (Utilities|Casting|CastToBP_MainPS (Variables|/Script/Engine.Controller|GetPlayerState ExitingController)))
  (Utilities|IsValid _asbp_main_ps
    (:Is%20Valid
      (bind _asbp_gi (Utilities|Casting|CastToBP_GI (Game|GetGameInstance)))
      (Utilities|IsValid _asbp_gi
        (:Is%20Valid
          (Default|SetUIDMainEmpty _asbp_gi (Variables|/Game/Blueprints/System/Main/BP_MainPS.BP_MainPS_C|GetUID _asbp_main_ps))
          (bind _asbp_main_pc (Utilities|Casting|CastToBP_MainPC (Game|GetPlayerController 0)))
          (Default|LogOutSubWidget _asbp_main_pc (Variables|/Game/Blueprints/System/Main/BP_MainPS.BP_MainPS_C|GetUID _asbp_main_ps))
          (Math|Integer|DecrementInt _playercount
            (:%20%20
              (if (!= _playercount 0)
                (Variables|Default|SetBulletDamage (/ (Variables|Default|GetBaseBulletDamage) (Math|Conversions|ToFloat(Integer) _playercount)))))))))))

(event EventPostLogin
  (params (NewPlayer :type Player%20Controller%20Object%20Reference))
  ;[1 1 1] OnPostLogin
  ;;[1 1 1] PlayerState UID 세팅
  (bind _asbp_main_ps (Utilities|Casting|CastToBP_MainPS (Variables|/Script/Engine.Controller|GetPlayerState NewPlayer)))
  (Default|SetInfo _asbp_main_ps)
  (bind _asbp_gi (Utilities|Casting|CastToBP_GI (Game|GetGameInstance)))
  ;[1 1 0] GameInstance에서 이 옵션이 켜져 있으면 첫번째 플레이어는 Octo로 나온다
  (if (Variables|/Game/Blueprints/Public/BP_GI.BP_GI_C|GetDebugUID0IsOcto _asbp_gi)
    (if (== (Variables|/Game/Blueprints/System/Main/BP_MainPS.BP_MainPS_C|GetUID _asbp_main_ps) 0)
      (bind _asbp_main_pc (Utilities|Casting|CastToBP_MainPC NewPlayer))
      (Variables|/Game/Blueprints/System/Main/BP_MainPC.BP_MainPC_C|SetRoleState _asbp_main_pc "NewEnumerator0")))
  (bind _isoctopus (Default|SetRoleState _asbp_main_ps))
  (if _isoctopus
    (bind _returnvalue (CallFunction|GetInitialPosition NewPlayer))
    (bind _returnvalue_2 (Game|SpawnActorfromClass "/Game/Blueprints/Octopus/BP_VRPawnMain.BP_VRPawnMain_C" _returnvalue "AlwaysSpawn" 0 0))
    (Variables|/Game/Blueprints/Octopus/BP_VRPawnMain.BP_VRPawnMain_C|SetInitLoading _returnvalue_2 true)
    (Pawn|Possess NewPlayer _returnvalue_2)
    (else
      ;;[1 1 0] 1p가 헌터일때
      (bind _asbp_main_pc_2 (Utilities|Casting|CastToBP_MainPC NewPlayer))
      (Utilities|IsValid _asbp_main_pc_2
        (:Is%20Valid
          (if (Pawn|IsLocalPlayerController _asbp_main_pc_2)
            (bind _asbp_gi_2 (Utilities|Casting|CastToBP_GI (Game|GetGameInstance)))
            (bind _returnvalue_3 (CallFunction|GetInitialPosition _asbp_main_pc_2))
            (bind _returnvalue_4 (Game|SpawnActorfromClass (Variables|/Game/Blueprints/Public/BP_GI.BP_GI_C|GetDefaultHunterClass _asbp_gi_2) _returnvalue_3 "AlwaysSpawn" 0 0))
            (Pawn|Possess _asbp_main_pc_2 _returnvalue_4)))))))

(fn ConstructionScript)

(fn GetHunterSpawnPoints
  (if (> (Utilities|Array|Length (Variables|Default|GetHunterRespawnPoints)) 0)
    _
    (else
      (bind _outactors (Actor|GetAllActorsOfClass "/Game/Blueprints/System/Main/BP_RespawnArea.BP_RespawnArea_C"))
      (Variables|Default|SetHunterRespawnPoints _outactors)))
  (Utilities|Array|Shuffle (Variables|Default|GetHunterRespawnPoints))
  (for _array_element (Variables|Default|GetHunterRespawnPoints)
    (bind _avaliable_ (Default|Avaliable _array_element))
    (if _avaliable_
      (bind _respawntransform (Default|GetRespawnPoint _array_element))
      (return _respawntransform)))
  ;[1 1 1] 모든 리스폰 포인트가 사용 불가능한 경우 - 맨 윗층에서 리스폰
  (bind _outactors_2 (Actor|GetAllActorswithTag "FinalSpawnPoint"))
  (bind _asbp_respawn_area (Utilities|Casting|CastToBP_RespawnArea (Utilities|Array|Get(acopy) _outactors_2 (Math|Random|RandomIntegerinRange 0 (- (Utilities|Array|Length _outactors_2) 1)))))
  (bind _respawntransform_2 (Default|GetRespawnPoint _asbp_respawn_area))
  (return _respawntransform_2))

(fn OnRepRemainRespawnNumber)

(fn GetInitialPosition
  (params (PlayerController :type Player%20Controller%20Object%20Reference))
  (bind _asbp_main_gs (Utilities|Casting|CastToBP_MainGS (Game|GetGameState)))
  (switch Utilities|FlowControl|Switch|SwitchonEMainGameState (Variables|/Script/OctoPrototype.MainGS|GetCurrentGameState _asbp_main_gs)
    (:Initialize
      (bind _outactors (Actor|GetAllActorswithTag "OctoLoading"))
      (return (Transformation|GetActorTransform (Utilities|Array|Get(acopy) _outactors))))
    (:Playing
      (bind _asbp_main_ps (Utilities|Casting|CastToBP_MainPS (Variables|/Script/Engine.Controller|GetPlayerState PlayerController)))
      (if (Utilities|Enum|Equal(Enum) (Variables|/Game/Blueprints/System/Main/BP_MainPS.BP_MainPS_C|GetRoleState _asbp_main_ps) "NewEnumerator0")
        (bind _outactors_2 (Actor|GetAllActorswithTag "OctoStart"))
        (return (Transformation|GetActorTransform (Utilities|Array|Get(acopy) _outactors_2)))
        (else
          (bind _respawntransform (CallFunction|GetHunterSpawnPoints))
          (return _respawntransform))))))