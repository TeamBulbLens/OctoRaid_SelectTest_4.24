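; BP_Barrior_Banner is a barrier wall prop whose look is configured through Blueprint variables, with no runtime logic.
; Its construction script creates a dynamic instance of M_Barrior_Wall on the SMBarriorWall mesh and stores it as MIBarriorWall.
; A sequence then pushes the variables into that instance by group: opacity mask texture, two colors, panning, UV tiling, and Fresnel, rim and distance-fade settings.
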(event EventBeginPlay)

(event Collision|EventActorBeginOverlap
  (params (OtherActor :type Actor%20Object%20Reference)))

(event EventTick
  (params (DeltaSeconds :type Float%20%28single-precision%29)))

(fn ConstructionScript
  (bind _returnvalue (Rendering|Material|CreateDynamicMaterialInstance (Variables|Default|GetSM_Barrior_Wall) 0 "/Game/AssetContents/Neon_Materials/Materials/M_Barrior_Wall/M_Barrior_Wall.M_Barrior_Wall" "M_Barrior_Wall" :!class /Script/Engine.PrimitiveComponent))
  (Variables|Default|SetMI_Barrior_Wall _returnvalue)
  (Utilities|FlowControl|Sequence
    (:then_0
      ;[1 1 1 1 28] Textures
      (Rendering|Material|SetTextureParameterValue (Variables|Default|GetMI_Barrior_Wall) "Opacity Mask" (Variables|Textures|GetOpacity%20Mask)))
    (:then_1
      ;[1 1 1 1 28] Opacity, Color, Emissive
      (Rendering|Material|SetVectorParameterValue (Variables|Default|GetMI_Barrior_Wall) "Color 1" (Variables|Color|GetColor%201) :!class /Script/Engine.MaterialInstanceDynamic)
      (Rendering|Material|SetVectorParameterValue (Variables|Default|GetMI_Barrior_Wall) "Color 2" (Variables|Color|GetColor%202) :!class /Script/Engine.MaterialInstanceDynamic))
    (:then_2
      ;[1 1 1 1 28] Panners
      (Rendering|Material|SetScalarParameterValue (Variables|Default|GetMI_Barrior_Wall) "X Panner" (Variables|Panner|GetX_Panner) :!class /Script/Engine.MaterialInstanceDynamic)
      (Rendering|Material|SetScalarParameterValue (Variables|Default|GetMI_Barrior_Wall) "Y Panner" (Variables|Panner|GetY_Panner) :!class /Script/Engine.MaterialInstanceDynamic))
    (:then_3
      ;[1 1 1 1 28] UV Tiling
      (Rendering|Material|SetScalarParameterValue (Variables|Default|GetMI_Barrior_Wall) "U Tiling" (Variables|Panner|GetU%20Tiling) :!class /Script/Engine.MaterialInstanceDynamic)
      (Rendering|Material|SetScalarParameterValue (Variables|Default|GetMI_Barrior_Wall) "V Tiling" (Variables|Panner|GetV%20Tiling) :!class /Script/Engine.MaterialInstanceDynamic))
    (:then_4
      ;[1 1 1 1 28] Fresnel
      (Rendering|Material|SetScalarParameterValue (Variables|Default|GetMI_Barrior_Wall) "Fresnel" (Variables|Color|GetFresnel) :!class /Script/Engine.MaterialInstanceDynamic)
      (Rendering|Material|SetScalarParameterValue (Variables|Default|GetMI_Barrior_Wall) "Rim Contrast" (Variables|Color|GetRim%20Contrast) :!class /Script/Engine.MaterialInstanceDynamic)
      (Rendering|Material|SetScalarParameterValue (Variables|Default|GetMI_Barrior_Wall) "Distance Fade" (Variables|Color|GetDistance%20Fade) :!class /Script/Engine.MaterialInstanceDynamic))))