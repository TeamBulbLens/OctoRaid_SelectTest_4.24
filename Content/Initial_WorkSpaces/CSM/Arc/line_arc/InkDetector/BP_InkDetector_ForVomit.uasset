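; BP_InkDetector_ForVomit is an ink hit detector, apparently for a vomit attack, that slows players it touches.
; Any overlap with HitCollision spawns an explosion particle at the collision's location.
; If the other actor is BP_PlayerCharacter_SN, it passes the debuff duration and effect percent, enables timed buffs and calls SlowDebuffsOn.
; The actor-destroy, ink explosion spawn and older character-cast branches are disconnected.
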(event OnComponentBeginOverlap(HitCollision)
  (params (OverlappedComponent :type Primitive%20Component%20Object%20Reference) (OtherActor :type Actor%20Object%20Reference) (OtherComp :type Primitive%20Component%20Object%20Reference) (OtherBodyIndex :type Integer) (bFromSweep :type Boolean) (SweepResult :type Hit%20Result%20Structure%20%28by%20ref%29))
  (Effects|SpawnEmitteratLocation "/Game/Initial_WorkSpaces/CSM/Arc/StarterContent/Particles/P_Explosion.P_Explosion" (Transformation|GetWorldLocation (Variables|Default|GetHitCollision)))
  (bind _asbp_player_character_sn (Utilities|Casting|CastToBP_PlayerCharacter_SN OtherActor))
  (Utilities|FlowControl|Sequence
    (:then_0
      (Variables|/Game/Blueprints/SN/Blueprints_SN/BP_PlayerCharacter_SN.BP_PlayerCharacter_SN_C|SetBuffsTimeSet _asbp_player_character_sn (Variables|Default|GetDebuffTime)))
    (:then_1
      (Variables|/Game/Blueprints/SN/Blueprints_SN/BP_PlayerCharacter_SN.BP_PlayerCharacter_SN_C|SetBuffsEffectPercentSet _asbp_player_character_sn (Variables|Default|GetBuffEffectPercent)))
    (:then_2
      (Variables|/Game/Blueprints/SN/Blueprints_SN/BP_PlayerCharacter_SN.BP_PlayerCharacter_SN_C|SetUseBuffsTime? _asbp_player_character_sn true))
    (:then_3
      (Default|SlowDebuffson _asbp_player_character_sn))))

(event EventBeginPlay
  (|CallParentFunction))

(event Collision|EventActorBeginOverlap
  (params (OtherActor :type Actor%20Object%20Reference))
  (|CallParentFunction OtherActor) ; 지금 이 노드는 비활성 상태입니다. \n핀을 끌어서 다른 노드를 연결하면 활성화됩니다.
)

(event EventTick
  (params (DeltaSeconds :type Float%20%28single-precision%29))
  (|CallParentFunction DeltaSeconds) ; 지금 이 노드는 비활성 상태입니다. \n핀을 끌어서 다른 노드를 연결하면 활성화됩니다.
)

(fn ConstructionScript
  (|CallParentFunction))